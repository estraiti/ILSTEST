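; Unit Blueprint that displays health and stamina bars through its Widget component.
; CreateWidgets enables actor Tick, then adds two equally filled WID_StatusBar widgets, red for health and green for stamina, to the component's vertical container.
; Tick polls the AttributeSet every frame and pushes current and max values into both bars.
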(event `self.ReceiveTick`
  (params (DeltaSeconds :type "Float (single-precision)"))
  (bind _attributeset (`self.AttributeSet`))
  (bind _attributeset_2 (`self.AttributeSet`))
  (`/Game/LISTestContent/UI/WID_StatusBar.SetValues` (`self.HealthBar`) (`.CurrentValue` (break `GameplayAttributeData` (`ILS_AttributeSet.Health` _attributeset))) (`.CurrentValue` (break `GameplayAttributeData` (`ILS_AttributeSet.MaxHealth` _attributeset))))
  (`/Game/LISTestContent/UI/WID_StatusBar.SetValues` (`self.StaminaBar`) (`.CurrentValue` (break `GameplayAttributeData` (`ILS_AttributeSet.Stamina` _attributeset_2))) (`.CurrentValue` (break `GameplayAttributeData` (`ILS_AttributeSet.MaxStamina` _attributeset_2)))))

(fn `CreateWidgets`
  (`self.SetActorTickEnabled` true)
  (bind _aswid_vertical_container (cast `/Game/LISTestContent/UI/Wid_VerticalContainer` (`WidgetComponent.GetWidget` (`self.Widget`))))
  (set `self.VerticalContainer` _aswid_vertical_container)
  (bind _returnvalue (`|CreateWidget` "/Game/LISTestContent/UI/WID_StatusBar.WID_StatusBar_C"))
  (bind _output_get (set `self.HealthBar` _returnvalue))
  (`/Game/LISTestContent/UI/Wid_VerticalContainer.AddChild` (`self.VerticalContainer`) _output_get)
  (`VerticalBoxSlot.SetSize` (`WidgetLayoutLibrary.SlotAsVerticalBoxSlot` _output_get) (make `SlateChildSize` 1.0))
  (`/Game/LISTestContent/UI/WID_StatusBar.SetBarColor` (`self.HealthBar`) (struct :`R` 1.0 :`B` 0.006324 :`A` 1.0))
  (bind _returnvalue_2 (`|CreateWidget` "/Game/LISTestContent/UI/WID_StatusBar.WID_StatusBar_C"))
  (bind _output_get_2 (set `self.StaminaBar` _returnvalue_2))
  (`/Game/LISTestContent/UI/Wid_VerticalContainer.AddChild` (`self.VerticalContainer`) _output_get_2)
  (`VerticalBoxSlot.SetSize` (`WidgetLayoutLibrary.SlotAsVerticalBoxSlot` _output_get_2) (make `SlateChildSize` 1.0))
  (`/Game/LISTestContent/UI/WID_StatusBar.SetBarColor` (`self.StaminaBar`) (struct :`G` 1.0 :`A` 1.0)))

(fn `UserConstructionScript`)