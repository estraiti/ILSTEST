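; Player unit Blueprint that shows on-screen health and stamina bars for the player.
; BeginPlay creates a vertical container widget anchored to the bottom-left of the viewport and fills it with two equally sized status bar widgets, red for health and green for stamina.
; Tick polls the AttributeSet and pushes current and maximum Health and Stamina values into the bars every frame, rather than reacting to attribute changes.
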(event `self.ReceiveBeginPlay`
  (bind _verticalcontainer (`self.VerticalContainer`))
  (bind _returnvalue (`|CreateWidget` "/Game/LISTestContent/UI/Wid_VerticalContainer.Wid_VerticalContainer_C"))
  (bind _output_get (set `self.VerticalContainer` _returnvalue))
  (`UserWidget.SetDesiredSizeInViewport` _output_get (500.0 100.0))
  (`UserWidget.AddToViewport` _verticalcontainer 0)
  (`UserWidget.SetPositionInViewport` _verticalcontainer (50.0 -50.0) false)
  (`UserWidget.SetAnchorsInViewport` _verticalcontainer (make `Anchors` (0.0 1.0) (0.0 1.0)))
  (`UserWidget.SetAlignmentInViewport` _verticalcontainer (0.0 1.0))
  (bind _returnvalue_2 (`|CreateWidget` "/Game/LISTestContent/UI/WID_StatusBar.WID_StatusBar_C"))
  (bind _output_get_2 (set `self.HealthBar` _returnvalue_2))
  (`/Game/LISTestContent/UI/Wid_VerticalContainer.AddChild` (`self.VerticalContainer`) _output_get_2)
  (`VerticalBoxSlot.SetSize` (`WidgetLayoutLibrary.SlotAsVerticalBoxSlot` _output_get_2) (make `SlateChildSize` 1.0))
  (`/Game/LISTestContent/UI/WID_StatusBar.SetBarColor` (`self.HealthBar`) (struct :`R` 1.0 :`B` 0.006324 :`A` 1.0))
  (bind _returnvalue_3 (`|CreateWidget` "/Game/LISTestContent/UI/WID_StatusBar.WID_StatusBar_C"))
  (bind _output_get_3 (set `self.StaminaBar` _returnvalue_3))
  (`/Game/LISTestContent/UI/Wid_VerticalContainer.AddChild` (`self.VerticalContainer`) _output_get_3)
  (`VerticalBoxSlot.SetSize` (`WidgetLayoutLibrary.SlotAsVerticalBoxSlot` _output_get_3) (make `SlateChildSize` 1.0))
  (`/Game/LISTestContent/UI/WID_StatusBar.SetBarColor` (`self.StaminaBar`) (struct :`G` 1.0 :`A` 1.0)))

(event `self.ReceiveTick`
  (params (DeltaSeconds :type "Float (single-precision)"))
  (bind _attributeset (`self.AttributeSet`))
  (bind _attributeset_2 (`self.AttributeSet`))
  (`/Game/LISTestContent/UI/WID_StatusBar.SetValues` (`self.HealthBar`) (`.CurrentValue` (break `GameplayAttributeData` (`ILS_AttributeSet.Health` _attributeset))) (`.CurrentValue` (break `GameplayAttributeData` (`ILS_AttributeSet.MaxHealth` _attributeset))))
  (`/Game/LISTestContent/UI/WID_StatusBar.SetValues` (`self.StaminaBar`) (`.CurrentValue` (break `GameplayAttributeData` (`ILS_AttributeSet.Stamina` _attributeset_2))) (`.CurrentValue` (break `GameplayAttributeData` (`ILS_AttributeSet.MaxStamina` _attributeset_2)))))

(fn `UserConstructionScript`)